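; AI-controlled character Blueprint with hitboxes and a hurtbox, driven by a simple timed behavior loop.
; BeginPlay assigns collision channels and overlap responses to the boxes, reverses the forward vector and out direction, and disables both hitboxes.
; Tick passes game time to the perceived action manager, while a repeating timer alternates between crouching and uncrouching with a backward move.
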(event EventBeginPlay
  (bind _forehitbox (Variables|Default|GetforeHitbox))
  (bind _backhitbox (Variables|Default|GetbackHitbox))
  (bind _hurtbox (Variables|Default|GetHurtbox))
  (|CallParentFunction)
  (Collision|SetCollisionObjectType _forehitbox "ECC_GameTraceChannel3")
  (Collision|SetCollisionResponsetoChannel _forehitbox "ECC_GameTraceChannel2" "ECR_Overlap")
  (Collision|SetCollisionObjectType _backhitbox "ECC_GameTraceChannel3")
  (Collision|SetCollisionResponsetoChannel _backhitbox "ECC_GameTraceChannel2" "ECR_Overlap")
  (Collision|SetCollisionObjectType _hurtbox "ECC_GameTraceChannel4")
  (Collision|SetCollisionResponsetoChannel _hurtbox "ECC_GameTraceChannel1" "ECR_Overlap")
  (Variables|Default|SetforwardVector (* (Math|Vector|GetForwardVector (Variables|Default|GetCollider)) -1.0))
  (Variables|Default|SetoutDir -1.0)
  (CallFunction|SetHitbox false (Variables|Default|GetforeHitbox))
  (CallFunction|SetHitbox false (Variables|Default|GetbackHitbox)))

(event Collision|EventActorBeginOverlap
  (params (OtherActor :type Actor%20Object%20Reference)))

(event EventTick
  (params (DeltaSeconds :type Float%20%28single-precision%29))
  (|CallParentFunction DeltaSeconds)
  (Class|AIPercievedActionManager|SetGameTime (Variables|Default|GetAIPercievedActionManager) (Utilities|Time|GetGameTimeinSeconds))
  (bind _output_get (Variables|Default|Settimer (- (Variables|Default|Gettimer) DeltaSeconds)))
  (if (<= _output_get 0.0)
    (Variables|Default|Settimer 3.0)
    (if (Variables|Default|GetisCrouching)
      (CallFunction|ExecuteUncrouch)
      (CallFunction|ExecuteMoveBackward)
      (else
        (CallFunction|ExecuteCrouch)))))

(fn ConstructionScript
  (|CallParentFunction))