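; Base fighter character for a melee punching game, with movement, crouch, uppercut, hook, counter and block.
; A CharacterState machine on Tick drives movement, body lean and timed states, though Blocking has no Tick case.
; Timelines animate fists and pushback; punch hitboxes resolve against the victim's state: crouching blocks uppercuts, retreating blocks hooks, countering freezes the attacker and counter-punches.
; Player-style actions report to PercievedActionManager; missed counters self-freeze.
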(event Custom|ExecuteMoveForward
  (bind _percievedactionmanager (Variables|Default|GetpercievedActionManager))
  (if (Utilities|Enum|NotEqual(Enum) (Variables|Default|GetcharacterState) "NewEnumerator2")
    (Utilities|IsValid _percievedactionmanager
      (:Is%20Valid
        (Class|AIPercievedActionManager|RecieveAction _percievedactionmanager "Foward" self))
      (:Is%20Not%20Valid
        _))
    (Variables|Default|SetcharacterState "NewEnumerator2")
    (CallFunction|ExecuteUncrouch)))

(event Custom|ExecuteIdle
  (Variables|Default|SetcharacterState "NewEnumerator0"))

(event Custom|ExecuteHook
  (bind _characterstate (Variables|Default|GetcharacterState))
  (bind _percievedactionmanager (Variables|Default|GetpercievedActionManager))
  (if (Math|Boolean|ORBoolean (Utilities|Enum|Equal(Enum) _characterstate "NewEnumerator0") (Utilities|Enum|Equal(Enum) _characterstate "NewEnumerator2") (Utilities|Enum|Equal(Enum) _characterstate "NewEnumerator3"))
    (Utilities|IsValid _percievedactionmanager
      (:Is%20Valid
        (Class|AIPercievedActionManager|RecieveAction _percievedactionmanager "Hook" self))
      (:Is%20Not%20Valid
        _))
    (|ExecuteHookNode)))

(event Custom|ExecuteCrouch
  (bind _percievedactionmanager (Variables|Default|GetpercievedActionManager))
  (bind _characterstate (Variables|Default|GetcharacterState))
  (if (and (Math|Boolean|ORBoolean (Utilities|Enum|Equal(Enum) _characterstate "NewEnumerator0") (Utilities|Enum|Equal(Enum) _characterstate "NewEnumerator2") (Utilities|Enum|Equal(Enum) _characterstate "NewEnumerator3")) (not (Variables|Default|GetisCrouching)))
    (Utilities|IsValid _percievedactionmanager
      (:Is%20Valid
        (Class|AIPercievedActionManager|RecieveAction _percievedactionmanager "Crouch" self))
      (:Is%20Not%20Valid
        _))
    (CallFunction|ExecuteIdle)
    (Variables|Default|SetisCrouching true)
    (bind _alpha (Timeline|CrouchTimeline PlayFromStart)
      (:Update
        (Transformation|SetRelativeTransform (Variables|Default|Getbody) (Math|Transform|Lerp(Transform) (Variables|Default|GetstandingTransform) (Variables|Default|GetcrouchingTransform) _alpha) false false)))))

(event Custom|ExecuteUppercut
  (bind _characterstate (Variables|Default|GetcharacterState))
  (bind _percievedactionmanager (Variables|Default|GetpercievedActionManager))
  (if (Math|Boolean|ORBoolean (Utilities|Enum|Equal(Enum) _characterstate "NewEnumerator0") (Utilities|Enum|Equal(Enum) _characterstate "NewEnumerator2") (Utilities|Enum|Equal(Enum) _characterstate "NewEnumerator3"))
    (Utilities|IsValid _percievedactionmanager
      (:Is%20Valid
        (Class|AIPercievedActionManager|RecieveAction _percievedactionmanager "Uppercut" self))
      (:Is%20Not%20Valid
        _))
    (|ExecuteUppercutNode)))

(event Custom|ExecuteCounter
  (bind _percievedactionmanager (Variables|Default|GetpercievedActionManager))
  (if (Math|Boolean|ORBoolean (Utilities|Enum|Equal(Enum) (Variables|Default|GetcharacterState) "NewEnumerator0") (Utilities|Enum|Equal(Enum) (Variables|Default|GetcharacterState) "NewEnumerator2") (Utilities|Enum|Equal(Enum) (Variables|Default|GetcharacterState) "NewEnumerator3"))
    (Utilities|IsValid _percievedactionmanager
      (:Is%20Valid
        (Class|AIPercievedActionManager|RecieveAction _percievedactionmanager "Counter" self))
      (:Is%20Not%20Valid
        _))
    (Variables|Default|SetcharacterState "NewEnumerator5")
    (Variables|Default|SetstateTimer 0.9)
    (Variables|Default|SetflashTimer 0.08)
    (Variables|Default|SetflashActive true)
    (Rendering|Material|SetMaterial (Variables|Default|Getbody) 0 "/Game/Character/CounterColor.CounterColor")
    (if (Variables|Default|GetisCrouching)
      (CallFunction|ExecuteUncrouch))))

(event Custom|ExecuteUncrouch
  (if (Variables|Default|GetisCrouching)
    (Variables|Default|SetisCrouching false)
    (bind _alpha (Timeline|UncrouchTimeline PlayFromStart)
      (:Update
        (Transformation|SetRelativeTransform (Variables|Default|Getbody) (Math|Transform|Lerp(Transform) (Variables|Default|GetcrouchingTransform) (Variables|Default|GetstandingTransform) _alpha) false false)))))

(event Custom|ExecuteFrozen
  (params (frozenTime :type Float%20%28single-precision%29))
  (Variables|Default|SetcharacterState "NewEnumerator9")
  (Variables|Default|SetstateTimer frozenTime))

(event Custom|ExecuteMoveBackward
  (bind _percievedactionmanager (Variables|Default|GetpercievedActionManager))
  (if (Utilities|Enum|NotEqual(Enum) (Variables|Default|GetcharacterState) "NewEnumerator3")
    (Utilities|IsValid _percievedactionmanager
      (:Is%20Valid
        (Class|AIPercievedActionManager|RecieveAction _percievedactionmanager "Backward" self))
      (:Is%20Not%20Valid
        _))
    (Variables|Default|SetcharacterState "NewEnumerator3")
    (CallFunction|ExecuteUncrouch)))

(event Custom|LerpFistsToOrigin
  (Variables|Default|SetforeFistStart (Variables|/Script/Engine.SceneComponent|GetRelativeLocation (Variables|Default|GetforeFist)))
  (Variables|Default|SetbackFistStart (Variables|/Script/Engine.SceneComponent|GetRelativeLocation (Variables|Default|GetbackFist)))
  (bind _dist (Timeline|LerpFistsTimeline PlayFromStart)
    (:Update
      (Transformation|SetRelativeLocation (Variables|Default|GetforeFist) (Math|Vector|Lerp(Vector) (Variables|Default|GetforeFistStart) "0, 0, 0" _dist) false false)
      (Transformation|SetRelativeLocation (Variables|Default|GetbackFist) (Math|Vector|Lerp(Vector) (Variables|Default|GetbackFistStart) "0, 0, 0" _dist) false false))))

(event Custom|ExecuteCounterPunch
  (|ExecuteCounterPunchNode))

(event Custom|ExecuteBlock
  (bind _collider (Variables|Default|GetCollider))
  (CallFunction|LerpFiststoOrigin)
  (Variables|Default|SetcharacterState "NewEnumerator10")
  (Variables|Default|SetstateTimer 0.4)
  (Variables|Default|SetpushBackStart (Transformation|GetWorldLocation _collider))
  (bind _dist (Timeline|BlockingPushBack PlayFromStart)
    (:Update
      (Transformation|SetWorldLocation _collider (+ (Variables|Default|GetpushBackStart) (* (Variables|Default|GetforwardVector) (* _dist -1.0 65.0))) true false))))

(event Custom|ExecuteDamaged
  (params (newKnockbackVel :type Float%20%28single-precision%29))
  (bind _collider (Variables|Default|GetCollider))
  (CallFunction|LerpFiststoOrigin)
  (Variables|Default|SetknockbackVelocity newKnockbackVel)
  (Variables|Default|SetcharacterState "NewEnumerator6")
  (Variables|Default|SetstateTimer 0.4)
  (Variables|Default|SetflashTimer 0.08)
  (Variables|Default|SetflashActive true)
  (Rendering|Material|SetMaterial (Variables|Default|Getbody) 0 "/Game/Character/DamagedColor.DamagedColor")
  (Variables|Default|SetpushBackStart (Transformation|GetWorldLocation _collider))
  (bind _dist (Timeline|DamagedPushBack PlayFromStart)
    (:Update
      (Transformation|SetWorldLocation _collider (+ (Variables|Default|GetpushBackStart) (* (Variables|Default|GetforwardVector) (* _dist -1.0 newKnockbackVel))) true false))))

(event EventBeginPlay)

(event Collision|EventActorBeginOverlap
  (params (OtherActor :type Actor%20Object%20Reference)))

(event EventTick
  (params (DeltaSeconds :type Float%20%28single-precision%29))
  (switch Utilities|FlowControl|Switch|SwitchonCharacterState (Variables|Default|GetcharacterState)
    (:NewEnumerator0
      (CallFunction|PitchtoZero DeltaSeconds))
    (:NewEnumerator2
      (|MoveForward DeltaSeconds))
    (:NewEnumerator3
      (|MoveBackward DeltaSeconds))
    (:NewEnumerator4
      (CallFunction|PitchtoZero DeltaSeconds))
    (:NewEnumerator7
      (CallFunction|PitchtoZero DeltaSeconds))
    (:NewEnumerator5
      (CallFunction|PitchtoZero DeltaSeconds)
      (|CounterNode DeltaSeconds))
    (:NewEnumerator8
      (CallFunction|PitchtoZero DeltaSeconds))
    (:NewEnumerator6
      (CallFunction|PitchtoZero DeltaSeconds)
      (|Damaged DeltaSeconds))
    (:NewEnumerator9
      (|FrozenNode DeltaSeconds))))

(fn ConstructionScript)

(fn PitchtoZero
  (params (delta :type Float%20%28single-precision%29))
  (bind _body (Variables|Default|Getbody))
  (bind _relativerotation (Variables|/Script/Engine.SceneComponent|GetRelativeRotation _body))
  (bind (_roll _pitch _yaw) (Math|Rotator|BreakRotator _relativerotation))
  (bind _returnvalue (Math|Float|Absolute(Float) _pitch))
  (if (> _returnvalue 0.75)
    (Transformation|SetRelativeRotation (Variables|Default|Getbody) (Math|Rotator|MakeRotator _roll (+ (* 6e+01 delta (/ _pitch _returnvalue) -1.0) _pitch) _yaw) false false)
    (else
      (Transformation|SetRelativeRotation (Variables|Default|Getbody) (Math|Rotator|MakeRotator _roll 0.0 _yaw) false false))))

(fn SetHitbox
  (params (active :type Boolean) (hitbox :type Sphere%20Component%20Object%20Reference))
  (if active
    (Collision|SetCollisionEnabled hitbox "QueryOnly")
    (else
      (Collision|SetCollisionEnabled hitbox "NoCollision"))))