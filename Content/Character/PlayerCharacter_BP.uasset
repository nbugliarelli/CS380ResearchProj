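; Player-controlled fighter Blueprint with keyboard-driven uppercut, hook, counter, crouch and forward/backward movement.
; Key events only set button flags; Tick runs HandleInput before the parent Tick.
; In three allowed CharacterState values, HandleInput calls Execute actions by priority: counter, hook, uppercut, crouch changes, then walking or idle, with no walking while crouched.
; BeginPlay puts hitboxes and hurtbox on custom overlap channels and starts both hitboxes disabled.
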(event EventBeginPlay
  (bind _forehitbox (Variables|Default|GetforeHitbox))
  (bind _backhitbox (Variables|Default|GetbackHitbox))
  (bind _hurtbox (Variables|Default|GetHurtbox))
  (Collision|SetCollisionObjectType _forehitbox "ECC_GameTraceChannel1")
  (Collision|SetCollisionResponsetoChannel _forehitbox "ECC_GameTraceChannel4" "ECR_Overlap")
  (Collision|SetCollisionObjectType _backhitbox "ECC_GameTraceChannel1")
  (Collision|SetCollisionResponsetoChannel _backhitbox "ECC_GameTraceChannel4" "ECR_Overlap")
  (Collision|SetCollisionObjectType _hurtbox "ECC_GameTraceChannel2")
  (Collision|SetCollisionResponsetoChannel _hurtbox "ECC_GameTraceChannel3" "ECR_Overlap")
  (Variables|Default|SetforwardVector (Math|Vector|GetForwardVector (Variables|Default|GetCollider)))
  (Variables|Default|SetoutDir 1.0)
  (CallFunction|SetHitbox false (Variables|Default|GetforeHitbox))
  (CallFunction|SetHitbox false (Variables|Default|GetbackHitbox)))

(event Collision|EventActorBeginOverlap
  (params (OtherActor :type Actor%20Object%20Reference)))

(event EventTick
  (params (DeltaSeconds :type Float%20%28single-precision%29))
  (CallFunction|HandleInput)
  (|CallParentFunction DeltaSeconds))

(event Input|KeyboardEvents|D
  (params (Key :type Key%20Structure :default "AnyKey"))
  (:Pressed
    (Variables|Default|SetforwardButton true))
  (:Released
    (Variables|Default|SetforwardButton false)))

(event Input|KeyboardEvents|A
  (params (Key :type Key%20Structure :default "AnyKey"))
  (:Pressed
    (Variables|Default|SetbackwardButton true))
  (:Released
    (Variables|Default|SetbackwardButton false)))

(event Input|KeyboardEvents|Up
  (params (Key :type Key%20Structure :default "AnyKey"))
  (:Pressed
    (Variables|Default|SetuppercutButton true))
  (:Released
    (Variables|Default|SetuppercutButton false)))

(event Input|KeyboardEvents|S
  (params (Key :type Key%20Structure :default "AnyKey"))
  (:Pressed
    (Variables|Default|SetcrouchButton true))
  (:Released
    (Variables|Default|SetcrouchButton false)))

(event Input|KeyboardEvents|Down
  (params (Key :type Key%20Structure :default "AnyKey"))
  (:Pressed
    (Variables|Default|SethookButton true))
  (:Released
    (Variables|Default|SethookButton false)))

(event Input|KeyboardEvents|Left
  (params (Key :type Key%20Structure :default "AnyKey"))
  (:Pressed
    (Variables|Default|SetcounterButton true))
  (:Released
    (Variables|Default|SetcounterButton false)))

(fn ConstructionScript
  (|CallParentFunction))

(fn HandleInput
  (bind _characterstate (Variables|Default|GetcharacterState))
  (if (Math|Boolean|ORBoolean (Utilities|Enum|Equal(Enum) _characterstate "NewEnumerator0") (Utilities|Enum|Equal(Enum) _characterstate "NewEnumerator2") (Utilities|Enum|Equal(Enum) _characterstate "NewEnumerator3"))
    (if (Variables|Default|GetcounterButton)
      (CallFunction|ExecuteCounter)
      (elif (Variables|Default|GethookButton)
        (CallFunction|ExecuteHook)
        (elif (Variables|Default|GetuppercutButton)
          (CallFunction|ExecuteUppercut)
          (elif (and (Variables|Default|GetcrouchButton) (not (Variables|Default|GetisCrouching)))
            (CallFunction|ExecuteCrouch)
            (CallFunction|ExecuteIdle)
            (elif (and (not (Variables|Default|GetcrouchButton)) (Variables|Default|GetisCrouching))
              (CallFunction|ExecuteUncrouch)
              (if (Variables|Default|GetforwardButton) :!label _label
                (if (Variables|Default|GetbackwardButton)
                  (CallFunction|ExecuteIdle)
                  (else
                    (CallFunction|ExecuteMoveForward)))
                (elif (Variables|Default|GetbackwardButton)
                  (CallFunction|ExecuteMoveBackward)
                  (else
                    (CallFunction|ExecuteIdle))))
              (elif (not (Variables|Default|GetisCrouching))
                (goto _label)))))))))